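; CameraController is a character-based Blueprint that moves itself from the MoveRight and MoveUp input axes.
; Nonzero MoveRight adds movement input along world X and nonzero MoveUp along world Z, scaled by the axis value.
; Either axis at zero calls StopMovementImmediately on CharacterMovement.
; The repeated nested zero checks leave their cross-axis movement branches unreachable.
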(event `InputAxis|MoveRight`
  (params (AxisValue :type "Float (single-precision)"))
  (if (== AxisValue 0.0)
    (if (== (stale `InputAxis|MoveUp` AxisValue) 0.0)
      (`MovementComponent.StopMovementImmediately` (`self.CharacterMovement`) :!label _label)
      (else
        (`self.AddMovementInput` (0.0 0.0 5.0) (stale `InputAxis|MoveUp` AxisValue) :!label _label_2)))
    (else
      (`self.AddMovementInput` (5.0 0.0 0.0) AxisValue :!label _label_3))))

(event `InputAxis|MoveUp`
  (params (AxisValue :type "Float (single-precision)"))
  (if (== AxisValue 0.0)
    (if (== (stale `InputAxis|MoveRight` AxisValue) 0.0)
      (goto _label)
      (else
        (goto _label_3)))
    (else
      (goto _label_2))))

(fn `UserConstructionScript`)