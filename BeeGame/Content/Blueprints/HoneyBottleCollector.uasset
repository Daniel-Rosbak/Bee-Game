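; HoneyBottleCollector is a 2D worker that ferries bottles from finished HoneyPackers to the world center, earning money through WorldGenerator.
; Tick alternates searching and travelling, with a Carrying flag choosing pickup or delivery and swapping the flipbook.
; Delivery targets a temporary Tile spawned at the center and destroyed once money is added.
; Movement teleports along the normalized XZ direction at constant speed, pitching the actor by arctangent.
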(event `self.ReceiveBeginPlay`
  (set `self.Searching` true)
  (set `self.Carrying` false)
  (set `self.Speed` 40.0))

(event `self.ReceiveTick`
  (params (DeltaSeconds :type "Float (single-precision)"))
  (if (`self.Searching`)
    (if (`self.Carrying`)
      (`KismetSystemLibrary.PrintString` "house")
      (`self.GoToCenter`)
      (else
        (`KismetSystemLibrary.PrintString` "packer")
        (`self.LookForFullPacker` :!label _label)))
    (elif (>= (`KismetMathLibrary.Vector_Distance` (`self.K2_GetActorLocation` (`self.Target`)) (`self.K2_GetActorLocation`)) 32.0)
      (`self.Move` DeltaSeconds)
      (elif (`self.Carrying`)
        (bind _success (`/Game/Blueprints/World_generation.AddMoney` (`self.WorldGenerator`) 20))
        (if _success
          (`PaperFlipbookComponent.SetFlipbook` (`self.collector`) "/Game/Animations/HoneyBottleCollector_Empty_FB.HoneyBottleCollector_Empty_FB")
          (`self.K2_DestroyActor` (`self.Target`))
          (set `self.Carrying` false)
          (set `self.Searching` true :!label _label_2))
        (else
          (bind _ashoney_packer (cast `/Game/Blueprints/HoneyPacker` (`self.Target`)))
          (bind _success_2 (`/Game/Blueprints/HoneyPacker.RemoveBottle` _ashoney_packer))
          (if _success_2
            (`PaperFlipbookComponent.SetFlipbook` (`self.collector`) "/Game/Animations/HoneyBottleCollector_Full_FB.HoneyBottleCollector_Full_FB")
            (set `self.Carrying` true)
            (goto _label_2)
            (else
              (goto _label))))))))

(fn `GoToCenter`
  (bind _returnvalue (`|SpawnActorFromClass` "/Game/Blueprints/Tile.Tile_C" (`KismetMathLibrary.MakeTransform` (0.0 -2.0 0.0)) "Undefined" "MultiplyWithRoot" null null))
  (set `self.Target` _returnvalue)
  (set `self.Searching` false))

(fn `LookForFullPacker`
  (bind _honeypackers (`self.HoneyPackers`))
  (`KismetSystemLibrary.PrintText` (`KismetTextLibrary.Conv_IntToText` (`KismetArrayLibrary.Array_Length` _honeypackers)))
  (for _array_element _honeypackers
    (if (`/Game/Blueprints/HoneyPacker.IsDone` _array_element)
      (set `self.Searching` false)
      (set `self.Target` _array_element)
      (else
        (`KismetSystemLibrary.PrintString` "failed")))))

(fn `Move`
  (params (DeltaSeconds :type "Float (double-precision)"))
  (bind _returnvalue (`self.K2_GetActorLocation`))
  (bind _speed (`self.Speed`))
  (bind (_x _y _z) (`KismetMathLibrary.BreakVector3f` (- (`self.K2_GetActorLocation` (`self.Target`)) _returnvalue)))
  (bind _returnvalue_2 (`KismetMathLibrary.Sqrt` (+ (`KismetMathLibrary.Square` _x) (`KismetMathLibrary.Square` _z))))
  (`KismetSystemLibrary.PrintString` "move")
  (`self.K2_TeleportTo` (+ _returnvalue (* (`KismetMathLibrary.MakeVector` (* (/ _x _returnvalue_2) _speed) 0.0 (* (/ _z _returnvalue_2) _speed)) DeltaSeconds)) (`KismetMathLibrary.MakeRotator` 0.0 (`KismetMathLibrary.DegAtan` (/ _z _x)))))

(fn `UserConstructionScript`)