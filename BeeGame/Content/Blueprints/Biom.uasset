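; Biome Blueprint that handles the locked state of a map biome, marked with an overlay actor.
; BiomLocked spawns a BiomeOverlay at the stored center tile plus a layer offset, skipping the center biome, and keeps it as BiomLock.
; BiomUnLocked calls DestroyActor when that overlay reference is valid, and a setter supplies the center tile.
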(fn `BiomLocked`
  (if (not (== (`self.BiomID`) (`self.CenterBiomID`)))
    (bind _returnvalue (`|SpawnActorFromClass` "/Game/Blueprints/BiomeOverlay.BiomeOverlay_C" (`KismetMathLibrary.MakeTransform` (+ (`self.CenterTile`) (`self.Layer`))) "Undefined" "MultiplyWithRoot" null null))
    (set `self.BiomLock` _returnvalue)))

(fn `BiomUnLocked`
  (if (`KismetSystemLibrary.IsValid` (`self.BiomLock`))
    (`self.K2_DestroyActor`)))

(fn `Set Centertile`
  (params (`Center tile` :type "Vector Structure"))
  (set `self.CenterTile` `Center tile`))

(fn `UserConstructionScript`)