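; HoneySling is a Paper2D honey slinger machine that turns honey frames into honey and feeds it into a connected Pipe.
; AddHoneyFrame accepts two frames, the second starting a three-second production timer on Tick and revealing the flipbook.
; When done, it hides the flipbook, shows the full sprite and retries Pipe.AddHoney each tick until accepted, then RemoveHoney restores the idle sprite.
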(event `self.ReceiveBeginPlay`
  (set `self.Idle` "/Game/Sprites/Honey_Slinger_Idle_Sprite.Honey_Slinger_Idle_Sprite")
  (set `self.Full` "/Game/Sprites/Honey_Slinger_Full_Sprite.Honey_Slinger_Full_Sprite")
  (set `self.HoneyFrames` 0)
  (set `self.Producing` false)
  (set `self.ProductionTimer` 0.0))

(event `self.ReceiveTick`
  (params (DeltaSeconds :type "Float (single-precision)"))
  (bind _productiontimer (`self.ProductionTimer`))
  (if (`self.Producing`)
    (if (>= _productiontimer 3.0)
      (set `self.Producing` false)
      (set `self.IsDone` true)
      (`PaperFlipbookComponent.SetSpriteColor` (`self.PaperFlipbook`) (struct :`R` 1.0 :`G` 1.0 :`B` 1.0))
      (`PaperSpriteComponent.SetSpriteColor` (`self.PaperSprite`) (struct :`R` 1.0 :`G` 1.0 :`B` 1.0 :`A` 1.0))
      (set `self.HoneyFrames` 0)
      (`PaperSpriteComponent.SetSprite` (`self.PaperSprite`) (`self.Full`))
      (if (`KismetSystemLibrary.IsValid` (`self.Pipe`)) :!label _label
        (bind _success (`/Game/Blueprints/Pipe.AddHoney` (`self.Pipe`)))
        (if _success
          (`self.RemoveHoney`)))
      (else
        (set `self.ProductionTimer` (+ _productiontimer DeltaSeconds))))
    (elif (`self.IsDone`)
      (goto _label))))

(fn `AddHoneyFrame`
  (returns (Success :type Boolean))
  (switch `int` (`self.HoneyFrames`)
    (:`Default`
      (return false))
    (:`0`
      (set `self.HoneyFrames` 1)
      (return true))
    (:`1`
      (set `self.HoneyFrames` 0)
      (set `self.Producing` true)
      (set `self.ProductionTimer` 0.0)
      (`PaperFlipbookComponent.SetSpriteColor` (`self.PaperFlipbook`) (struct :`R` 1.0 :`G` 1.0 :`B` 1.0 :`A` 1.0))
      (`PaperSpriteComponent.SetSpriteColor` (`self.PaperSprite`) (struct :`R` 1.0 :`G` 1.0 :`B` 1.0 :`A` 1.0))
      (return true))))

(fn `RemoveHoney`
  (`PaperSpriteComponent.SetSprite` (`self.PaperSprite`) (`self.Idle`))
  (set `self.IsDone` false))

(fn `UserConstructionScript`)