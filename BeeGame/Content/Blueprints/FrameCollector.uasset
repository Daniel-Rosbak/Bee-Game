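; Paper2D frame collector that ferries honey frames from finished beehives to idle honey slings.
; Tick alternates between searching the hive or sling arrays, based on whether it carries a frame, and moving to the target.
; Movement teleports it along the XZ plane at constant speed, pitched toward the target.
; On arrival it removes or adds a frame, swaps the full or empty flipbook, and resumes searching, retrying the search if the transfer fails.
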(event `self.ReceiveBeginPlay`
  (set `self.Searching` true)
  (set `self.Carrying` false)
  (set `self.Speed` 40.0))

(event `self.ReceiveTick`
  (params (DeltaSeconds :type "Float (single-precision)"))
  (bind _target (`self.Target`))
  (bind _collector (`self.collector`))
  (if (`self.Searching`)
    (if (`self.Carrying`)
      (`self.LookForEmptyHoneySling` :!label _label)
      (else
        (`self.LookForFullBeeHive` :!label _label_2)))
    (elif (>= (`KismetMathLibrary.Vector_Distance` (`self.K2_GetActorLocation` (`self.Target`)) (`self.K2_GetActorLocation`)) 32.0)
      (`self.MoveTowardTarget` DeltaSeconds)
      (else
        (if (`self.Carrying`)
          (bind _ashoney_sling (cast `/Game/Blueprints/HoneySling` _target))
          (bind _success (`/Game/Blueprints/HoneySling.AddHoneyFrame` _ashoney_sling))
          (if _success
            (`PaperFlipbookComponent.SetFlipbook` _collector "/Game/Animations/HoneyFrameCollector_Empty_FB.HoneyFrameCollector_Empty_FB")
            (set `self.Carrying` false)
            (else
              (goto _label)))
          (else
            (bind _asbeehive (cast `/Game/Blueprints/Beehive` _target))
            (bind _success_2 (`/Game/Blueprints/Beehive.RemoveHoneyFrame` _asbeehive))
            (if _success_2
              (`PaperFlipbookComponent.SetFlipbook` _collector "/Game/Animations/HoneyFrameCollector_Full_FB.HoneyFrameCollector_Full_FB")
              (set `self.Carrying` true)
              (else
                (goto _label_2)))))
        (set `self.Searching` true)))))

(fn `LookForEmptyHoneySling`
  (for _array_element (`self.HoneySlings`)
    (if (`/Game/Blueprints/HoneySling.IsDone` _array_element)
      _
      (elif (not (`/Game/Blueprints/HoneySling.Producing` _array_element))
        (set `self.Searching` false)
        (set `self.Target` _array_element)))))

(fn `LookForFullBeeHive`
  (bind _beehives (`self.Beehives`))
  (`KismetSystemLibrary.PrintString` (`KismetStringLibrary.Conv_IntToString` (`KismetArrayLibrary.Array_Length` _beehives)))
  (for _array_element _beehives
    (if (`/Game/Blueprints/Beehive.IsDone` _array_element)
      (set `self.Searching` false)
      (set `self.Target` _array_element)
      (else
        (`KismetSystemLibrary.PrintString` "failed")))))

(fn `MoveTowardTarget`
  (params (DeltaSeconds :type "Float (double-precision)"))
  (bind _returnvalue (`self.K2_GetActorLocation`))
  (bind _speed (`self.Speed`))
  (bind (_x _y _z) (`KismetMathLibrary.BreakVector3f` (- (`self.K2_GetActorLocation` (`self.Target`)) _returnvalue)))
  (bind _returnvalue_2 (`KismetMathLibrary.Sqrt` (+ (`KismetMathLibrary.Square` _x) (`KismetMathLibrary.Square` _z))))
  (`self.K2_TeleportTo` (+ _returnvalue (* (`KismetMathLibrary.MakeVector` (* (/ _x _returnvalue_2) _speed) 0.0 (* (/ _z _returnvalue_2) _speed)) DeltaSeconds)) (`KismetMathLibrary.MakeRotator` 0.0 (+ (`KismetMathLibrary.DegAtan` (/ _z _x)) 90.0))))

(fn `UserConstructionScript`)