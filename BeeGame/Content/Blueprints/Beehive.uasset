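; Beehive is a 2D Paper2D Blueprint that produces honey over time, swapping between idle and full sprites.
; Tick accumulates elapsed time until it reaches the production speed, then flags the hive as done and shows the full sprite.
; RemoveHoneyFrame resets the flag, sprite and timer to restart production.
; CheckForFlowers runs on begin play and after each reset but is an empty stub.
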(event `self.ReceiveBeginPlay`
  (set `self.Idle` "/Game/Sprites/Beehive_Sprite.Beehive_Sprite")
  (set `self.Full` "/Game/Sprites/Beehive_full_Sprite.Beehive_full_Sprite")
  (set `self.IsDone` false)
  (set `self.ProductionTimer` 0.0)
  (set `self.ProductionSpeed` 15.0)
  (`self.CheckForFlowers`))

(event `self.ReceiveTick`
  (params (DeltaSeconds :type "Float (single-precision)"))
  (bind _productiontimer (`self.ProductionTimer`))
  (if (`self.IsDone`)
    _
    (elif (>= _productiontimer (`self.ProductionSpeed`))
      (set `self.IsDone` true)
      (`PaperSpriteComponent.SetSprite` (`self.PaperSprite`) (`self.Full`))
      (else
        (set `self.ProductionTimer` (+ _productiontimer DeltaSeconds))))))

(fn `CheckForFlowers`)

(fn `RemoveHoneyFrame`
  (set `self.IsDone` false)
  (`PaperSpriteComponent.SetSprite` (`self.PaperSprite`) (`self.Idle`))
  (set `self.ProductionTimer` 0.0)
  (`self.CheckForFlowers`))

(fn `UserConstructionScript`)