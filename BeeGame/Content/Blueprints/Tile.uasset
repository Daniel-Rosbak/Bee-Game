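; Map tile actor built on Paper2D that shows a grass, sand or ice biome and can hold flowers, a farmhouse and bees.
; Separate functions swap sprites on the tile, flower and house components and toggle the bee flipbook, nudging flowers and house along Y for layering.
; Flower spawning requires the center-biome flag and skips the center tile and hardcoded neighbor IDs.
; Destroying flowers removes their component and clears the bees.
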(event `self.ReceiveBeginPlay`)

(event `self.ReceiveTick`
  (params (DeltaSeconds :type "Float (single-precision)")))

(event `self.Tile.OnBeginCursorOver`
  (params (TouchedComponent :type "PrimitiveComponent Object Reference")))

(fn `checkIfContainsFlower`
  (returns (hasFlower :type Boolean))
  (return (`self.hasFlower`)))

(fn `DestroyFlowers`
  (if (`self.hasFlower`)
    (`ActorComponent.K2_DestroyComponent` (`self.Flower`))
    (set `self.hasFlower` false)
    (`self.RemoveBees`)))

(fn `FlowerType`
  (params (BiomType :type Integer))
  (bind _flower (`self.Flower`))
  (switch `int` BiomType
    (:`0`
      (`PaperSpriteComponent.SetSprite` _flower "/Game/Sprites/Flowers_Grass_Sprite.Flowers_Grass_Sprite"))
    (:`1`
      (`PaperSpriteComponent.SetSprite` _flower "/Game/Sprites/Flowers_Sand_Sprite.Flowers_Sand_Sprite"))
    (:`2`
      (`PaperSpriteComponent.SetSprite` _flower "/Game/Sprites/Flowers_Ice_Sprite.Flowers_Ice_Sprite"))))

(fn `MakeBees`
  (`PaperFlipbookComponent.SetFlipbook` (`self.Bees`) "/Game/Animations/Bees.Bees")
  (set `self.hasBees` true))

(fn `RemoveBees`
  (`PaperFlipbookComponent.SetFlipbook` (`self.Bees`) null)
  (set `self.hasBees` false))

(fn `SetTileType`
  (params (BiomType :type Integer))
  (bind _tile (`self.Tile`))
  (bind _output_get (set `self.BiomType` BiomType))
  (switch `int` _output_get
    (:`0`
      (`PaperSpriteComponent.SetSprite` _tile "/Game/Sprites/GrassTile_Sprite.GrassTile_Sprite"))
    (:`1`
      (`PaperSpriteComponent.SetSprite` _tile "/Game/Sprites/SandTile_Sprite.SandTile_Sprite"))
    (:`2`
      (`PaperSpriteComponent.SetSprite` _tile "/Game/Sprites/IceTile_Sprite.IceTile_Sprite"))))

(fn `Spawn house`
  (bind _house (`self.House`))
  (`PaperSpriteComponent.SetSprite` _house "/Game/Sprites/FarmHouse_Sprite.FarmHouse_Sprite")
  (set `self.FlowerLayer` (0.0 1.0 0.0))
  (`SceneComponent.K2_SetWorldTransform` _house (`KismetMathLibrary.MakeTransform` (+ (.location (`SceneComponent.K2_GetComponentToWorld` _house)) (`self.FlowerLayer`))) false false))

(fn `SpawnFlowers`
  (params (BiomType :type Integer) (CenterBiom :type Boolean))
  (bind _array (`|MakeArray` 50 51 62 64 75 76))
  (bind _flower (`self.Flower`))
  (if (`self.hasFlower`)
    _
    (elif CenterBiom
      (if (not (`self.CenterTile`))
        (set `self.TIlesNearCenter` _array)
        (if (not (`KismetArrayLibrary.Array_Contains` _array (`self.TileID`)))
          (bind _output_get (set `self.FlowerLayer` (0.0 1.0 0.0)))
          (`SceneComponent.K2_SetWorldTransform` _flower (`KismetMathLibrary.MakeTransform` (+ (.location (`SceneComponent.K2_GetComponentToWorld` _flower)) _output_get)) false false)
          (`self.FlowerType` BiomType)
          (set `self.hasFlower` true))))))

(fn `UserConstructionScript`)