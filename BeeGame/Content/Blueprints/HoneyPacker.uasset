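; Honey packer machine in a 2D Paper2D world that turns two units of honey into a removable bottle.
; AddHoney counts units and starts production on the second, and Tick runs a ten-second timer before showing the full sprite until RemoveBottle clears it.
; Sprite and flipbook alpha swap to show the working animation.
; FindPipe scans hex-grid neighbors among WorldGenerator placeables, and CheckPipes registers the packer on adjacent pipes.
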(event `self.ReceiveBeginPlay`
  (set `self.Idle` "/Game/Sprites/Honey_Packer_Idle_Sprite.Honey_Packer_Idle_Sprite")
  (set `self.Full` "/Game/Sprites/Honey_Packer_Full_Sprite.Honey_Packer_Full_Sprite")
  (set `self.Honey` 0)
  (set `self.Producing` false)
  (set `self.ProductionTimer` 0.0))

(event `self.ReceiveTick`
  (params (DeltaSeconds :type "Float (single-precision)"))
  (bind _productiontimer (`self.ProductionTimer`))
  (if (`self.Producing`)
    (if (>= _productiontimer 10.0)
      (set `self.Producing` false)
      (set `self.IsDone` true)
      (`PaperFlipbookComponent.SetSpriteColor` (`self.PaperFlipbook`) (struct :`R` 1.0 :`G` 1.0 :`B` 1.0))
      (`PaperSpriteComponent.SetSpriteColor` (`self.PaperSprite`) (struct :`R` 1.0 :`G` 1.0 :`B` 1.0 :`A` 1.0))
      (set `self.Honey` 0)
      (`PaperSpriteComponent.SetSprite` (`self.PaperSprite`) (`self.Full`))
      (else
        (set `self.ProductionTimer` (+ _productiontimer DeltaSeconds))))))

(fn `AddHoney`
  (returns (Success :type Boolean))
  (switch `int` (`self.Honey`)
    (:`Default`
      (return false))
    (:`0`
      (set `self.Honey` 1)
      (return true))
    (:`1`
      (set `self.Honey` 0)
      (set `self.Producing` true)
      (set `self.ProductionTimer` 0.0)
      (`PaperFlipbookComponent.SetSpriteColor` (`self.PaperFlipbook`) (struct :`R` 1.0 :`G` 1.0 :`B` 1.0 :`A` 1.0))
      (`PaperSpriteComponent.SetSpriteColor` (`self.PaperSprite`) (struct :`R` 1.0 :`G` 1.0 :`B` 1.0))
      (return true))))

(fn `CheckPipes`
  (for _array_element (`self.SurroundingPipes`)
    (if (== (`GameplayStatics.GetObjectClass` _array_element) "/Game/Blueprints/Pipe.Pipe_C")
      (`KismetSystemLibrary.PrintString` "PIPE!!!")
      (bind _aspipe (cast `/Game/Blueprints/Pipe` _array_element))
      (set `/Game/Blueprints/Pipe.Packer` self _aspipe))))

(fn `FindPipe`
  (bind _positions (`self.Positions`))
  (bind (_x _y _z) (`KismetMathLibrary.BreakVector3f` (`self.K2_GetActorLocation`)))
  (for _index (range -1 2)
    (for _index_2 (range -1 2)
      (bind _returnvalue (+ _index _index_2))
      (if (and (<= _returnvalue 1) (>= _returnvalue -1))
        (`KismetArrayLibrary.Array_Add` _positions (+ (* _index (48.0 0.0 32.0)) (* _index_2 (0.0 0.0 64.0)) (`KismetMathLibrary.MakeVector` _x 0.0 _z)))))
    (for _array_element (`/Game/Blueprints/World_generation.Placeables` (`self.WorldGenerator`))
      (if (`KismetArrayLibrary.Array_Contains` _positions (`KismetMathLibrary.MakeVector` (.x (`self.K2_GetActorLocation` _array_element)) 0.0 (.z (`self.K2_GetActorLocation` _array_element))))
        (`KismetArrayLibrary.Array_AddUnique` (`self.SurroundingPipes`) _array_element)))
    (`self.CheckPipes`)))

(fn `RemoveBottle`
  (returns (Success :type Boolean))
  (if (`self.IsDone`)
    (`PaperSpriteComponent.SetSprite` (`self.PaperSprite`) (`self.Idle`))
    (set `self.IsDone` false)
    (return true)
    (else
      (return false))))

(fn `UserConstructionScript`)