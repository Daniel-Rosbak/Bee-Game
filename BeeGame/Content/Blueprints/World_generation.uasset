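; World generator actor that builds hexagonal biomes of tiles and flowers on the XZ plane at BeginPlay, currently just the center biome.
; GenerateBiome uses nested axial-coordinate loops to spawn Biom actors and their Tiles, with type 0 at the center and random types elsewhere.
; Flowers matching the biome type scatter over random tile positions, using a set against duplicates and a center-tile check in the center biome.
; Each biome stores its positions, then gets BiomLocked.
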(event `self.ReceiveBeginPlay`
  (`self.GenerateBiome` 0 127 3))

(fn `GenerateBiome`
  (params (radiusFromCenterBiom :type Integer :default 10) (MaxNumOfFlowersPerBiom :type Integer :default 55) (NumOfdifferentBiomTypes :type Integer))
  (bind _returnvalue (* radiusFromCenterBiom -1))
  (bind _returnvalue_2 (+ 1 radiusFromCenterBiom))
  (bind _flowerposset (`self.flowerPosSet`))
  (for _index (range _returnvalue (+ radiusFromCenterBiom 1))
    (for _index_2 (range _returnvalue (+ radiusFromCenterBiom 1))
      (if (== _index 0)
        (if (== _index_2 0)
          (set `self.BiomType` 0)
          (else
            (set `self.BiomType` (`KismetMathLibrary.RandomInteger` NumOfdifferentBiomTypes) :!label _label)))
        (else
          (goto _label)))
      (bind _returnvalue_3 (+ _index_2 _index))
      (if (and (< _returnvalue_3 _returnvalue_2) (> _returnvalue_3 (* _returnvalue_2 -1)))
        (bind _output_get (set `self.RLarge` (624.0 0.0 32.0)))
        (bind _output_get_2 (set `self.QLarge` (288.0 0.0 640.0)))
        (bind _returnvalue_4 (`|SpawnActorFromClass` "/Game/Blueprints/Biom.Biom_C" (`KismetMathLibrary.MakeTransform` (0.0 0.0 0.0)) "Undefined" "MultiplyWithRoot" null null))
        (bind _output_get_3 (set `/Game/Blueprints/Biom.BiomID` (+ (`self.BiomID`) 1) _returnvalue_4))
        (set `self.BiomID` _output_get_3)
        (if (== _index 0)
          (if (== _index_2 0)
            (set `/Game/Blueprints/Biom.CenterBiomID` (`self.BiomID`) _returnvalue_4)))
        (for _index_3 (range -6 7)
          (for _index_4 (range -6 7)
            (bind _returnvalue_5 (+ _index_4 _index_3))
            (if (and (< _returnvalue_5 7) (> _returnvalue_5 -7))
              (bind _output_get_4 (set `self.RLittle` (0.0 0.0 64.0)))
              (bind _output_get_5 (set `self.QLittle` (48.0 0.0 32.0)))
              (bind _returnvalue_6 (+ (* _output_get_5 _index_3) (* _output_get_4 _index_4) (* _output_get _index) (* _output_get_2 _index_2)))
              (`KismetArrayLibrary.Array_Add` (`self.tilePosInBiom`) _returnvalue_6)
              (if (== _index_3 0)
                (if (== _index_4 0)
                  (`/Game/Blueprints/Biom.Set Centertile` _returnvalue_4 _returnvalue_6)))
              (bind _returnvalue_7 (`|SpawnActorFromClass` "/Game/Blueprints/Tile.Tile_C" (`KismetMathLibrary.MakeTransform` _returnvalue_6) "Undefined" "MultiplyWithRoot" null null))
              (`/Game/Blueprints/Tile.SetTileType` _returnvalue_7 (`self.BiomType`)))))
        (for _ (range (+ MaxNumOfFlowersPerBiom 1))
          (bind _output_get_6 (set `self.flowerPos` (0.0 1.0 0.0)))
          (if (== (`/Game/Blueprints/Biom.CenterBiomID` _returnvalue_4) (`self.BiomID`))
            (bind _returnvalue_8 (+ _output_get_6 (`KismetArrayLibrary.Array_Random` (`self.tilePosInBiom`))))
            (if (not (== (+ (`/Game/Blueprints/Biom.CenterTile` _returnvalue_4) _output_get_6) _returnvalue_8 :`ErrorTolerance` 0.0))
              (if (not (`BlueprintSetLibrary.Set_Contains` _flowerposset _returnvalue_8)) :!label _label_2
                (`BlueprintSetLibrary.Set_Add` _flowerposset _returnvalue_8)
                (bind _result (`BlueprintSetLibrary.Set_ToArray` (`self.flowerPosSet`)))
                (bind _output (`|GetArrayItem` _result (`KismetArrayLibrary.Array_LastIndex` _result)))
                (`KismetArrayLibrary.Array_Add` (`/Game/Blueprints/Biom.BiomFlowerPos` _returnvalue_4) _output)
                (bind _returnvalue_9 (`|SpawnActorFromClass` "/Game/Blueprints/Flowers.Flowers_C" (`KismetMathLibrary.MakeTransform` _output) "Undefined" "MultiplyWithRoot" null null))
                (`/Game/Blueprints/Flowers.SetFlowersType` _returnvalue_9 (`self.BiomType`))))
            (else
              (goto _label_2))))
        (set `/Game/Blueprints/Biom.BiomTilePos` (`self.tilePosInBiom`) _returnvalue_4)
        (`KismetArrayLibrary.Array_Clear` (`self.tilePosInBiom`))
        (`/Game/Blueprints/Biom.BiomLocked` _returnvalue_4)))))

(fn `UserConstructionScript`)